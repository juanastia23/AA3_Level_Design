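; Balcony light Blueprint that switches on and off as the player's cat character enters and leaves its trigger Box.
; Begin overlap, gated by LightOff, waits briefly, then applies an emissive yellow material to LightObject and raises RectLight intensity.
; End overlap, gated by a separate LightOn flag, waits longer, then restores the white material and zeroes the intensity.
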(event OnComponentBeginOverlap(Box)
  (params (OverlappedComponent :type Primitive%20Component%20Object%20Reference) (OtherActor :type Actor%20Object%20Reference) (OtherComp :type Primitive%20Component%20Object%20Reference) (OtherBodyIndex :type Integer) (bFromSweep :type Boolean) (SweepResult :type Hit%20Result%20Structure%20%28by%20ref%29))
  (Utilities|Casting|CastToBP_FirstPersonCharacter_Cat OtherActor)
  (if (Variables|Default|GetLight_Off?)
    (Utilities|FlowControl|Delay 0.5)
    (Rendering|Material|SetMaterial (Variables|Default|GetLight_Object) 0 "/Game/LevelPrototyping/Materials/MI_Blockout_Grid_Yellow_Emissive.MI_Blockout_Grid_Yellow_Emissive")
    (Rendering|Components|Light|SetIntensity (Variables|Default|GetRectLight) 2.5e+02)
    (Variables|Default|SetLight_Off? false)
    (else
      (Variables|Default|SetLight_On? true))))

(event OnComponentEndOverlap(Box)
  (params (OverlappedComponent :type Primitive%20Component%20Object%20Reference) (OtherActor :type Actor%20Object%20Reference) (OtherComp :type Primitive%20Component%20Object%20Reference) (OtherBodyIndex :type Integer))
  (Utilities|Casting|CastToBP_FirstPersonCharacter_Cat OtherActor)
  (if (Variables|Default|GetLight_On?)
    (Utilities|FlowControl|Delay 2.0)
    (Rendering|Material|SetMaterial (Variables|Default|GetLight_Object) 0 "/Game/LevelPrototyping/Materials/MI_Blockout_Custom_White.MI_Blockout_Custom_White")
    (Rendering|Components|Light|SetIntensity (Variables|Default|GetRectLight) 0.0)
    (Variables|Default|SetLight_Off? true)
    (else
      (Variables|Default|SetLight_On? false))))

(fn ConstructionScript)